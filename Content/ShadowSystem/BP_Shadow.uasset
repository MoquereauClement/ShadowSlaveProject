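; Shadow actor that glides across floors and walls as a surface-aligned decal, driven by input axes and view heading from SetShadowInput.
; Tick splits movement into short substeps, each tracing ahead, below, around outer edges, then back at its origin.
; Hits carry the forward vector onto the new normal, snap position and reorient the decal; losing contact triggers a downward reacquire.
; Older wall and ground trace logic in the EventGraph is disconnected.
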(event `self.ReceiveTick`
  (params (DeltaSeconds :type "Float (single-precision)"))
  (`self.TickShadowSurface` DeltaSeconds))

(event `self.ReceiveBeginPlay`
  (`self.AcquireShadowSurface`))

(event `TryDescendFromEdge`
  (`self.TickShadowSurface` (`GameplayStatics.GetWorldDeltaSeconds`)))

(fn `AcceptShadowContact`
  (bind _surfacenormal (`self.SurfaceNormal`))
  (bind _surfacenormal_2 (`self.SurfaceNormal`))
  (bind _z (.z _surfacenormal_2))
  (bind _returnvalue (< (`KismetMathLibrary.Abs` _z) 0.7))
  (bind _returnvalue_2 (`KismetMathLibrary.Normal` (`KismetMathLibrary.ProjectVectorOnToPlane` (`KismetMathLibrary.SelectVector` (`self.SurfaceForward`) (`KismetMathLibrary.GetForwardVector` (`self.InputHeading`)) _returnvalue) _surfacenormal_2)))
  (set `self.SurfaceForward` (`KismetMathLibrary.Quat_RotateVector` (`KismetMathLibrary.Quat_FindBetweenNormals` (`self.SurfaceNormal`) (`self.ProbeNormal`)) (`self.SurfaceForward`)))
  (set `self.SurfaceNormal` (`KismetMathLibrary.Normal` (`self.ProbeNormal`)))
  (set `self.SurfaceForward` _returnvalue_2)
  (set `self.HasSurface` true)
  (set `self.isOnWall` _returnvalue)
  (set `self.wallDetected` _returnvalue)
  (set `self.hasGround` (>= _z 0.7))
  (set `self.lastWallNormal` _surfacenormal)
  (`self.K2_SetActorLocation` (+ (`self.ProbePoint`) (* _surfacenormal (`self.SurfaceOffset`))))
  (`SceneComponent.K2_SetWorldRotation` (`self.ShadowDecal`) (`KismetMathLibrary.ComposeRotators` (`KismetMathLibrary.MakeRotator` (`self.ShadowArtworkRoll`)) (`KismetMathLibrary.MakeRotFromXZ` (* _surfacenormal_2 -1.0) _returnvalue_2)) false false))

(fn `AcquireShadowSurface`
  (bind _returnvalue (`self.K2_GetActorLocation`))
  (bind _ignoredactors (`self.IgnoredActors`))
  (`KismetArrayLibrary.Array_AddUnique` _ignoredactors (`GameplayStatics.GetPlayerPawn` 0))
  (`KismetArrayLibrary.Array_AddUnique` _ignoredactors (`self.GetOwner`))
  (`self.ProbeShadowSurface` (+ _returnvalue (0.0 0.0 100.0)) (+ _returnvalue (0.0 0.0 -1000.0)))
  (if (`self.ProbeHit`)
    (set `self.wallEdgeDetected` false)
    (`self.AcceptShadowContact`)
    (else
      (set `self.HasSurface` false)
      (set `self.hasGround` false)
      (set `self.isOnWall` false)
      (set `self.wallDetected` false))))

(fn `ProbeShadowSurface`
  (params (Start :type "Vector Structure") (End :type "Vector Structure"))
  (bind (_outhit _returnvalue) (`KismetSystemLibrary.LineTraceSingle` Start End "TraceTypeQuery1" true (`self.IgnoredActors`)))
  (set `self.ProbeHit` _returnvalue)
  (bind (_bblockinghit _binitialoverlap _time _distance _location _impactpoint _normal _impactnormal) (`GameplayStatics.BreakHitResult` _outhit))
  (set `self.ProbePoint` _impactpoint)
  (set `self.ProbeNormal` _impactnormal))

(fn `SetShadowInput`
  (params (RightInput :type "Float (double-precision)") (ForwardInput :type "Float (double-precision)") (ViewHeading :type "Rotator Structure"))
  (set `self.InputAxes` (`KismetMathLibrary.Vector_ClampSizeMax` (`KismetMathLibrary.MakeVector` RightInput ForwardInput) 1.0))
  (set `self.InputHeading` ViewHeading))

(fn `StepShadowSurface`
  (bind _probehit (`self.ProbeHit`))
  (bind _probedepth (`self.ProbeDepth`))
  (bind _surfacenormal (`self.SurfaceNormal`))
  (bind _returnvalue (* (`self.SurfaceNormal`) (`self.ProbeLift`)))
  (bind _returnvalue_2 (* (`self.SurfaceNormal`) _probedepth))
  (bind _returnvalue_3 (- (`self.StepCandidate`) _returnvalue_2))
  (bind _returnvalue_4 (- (`self.StepOrigin`) _returnvalue_2))
  (bind _returnvalue_5 (`KismetMathLibrary.Normal` (`KismetMathLibrary.ProjectVectorOnToPlane` (`KismetMathLibrary.SelectVector` (`self.SurfaceForward`) (`KismetMathLibrary.GetForwardVector` (`self.InputHeading`)) (< (`KismetMathLibrary.Abs` (.z _surfacenormal)) 0.7)) _surfacenormal)))
  (bind _returnvalue_6 (`KismetMathLibrary.Vector_ClampSizeMax` (+ (* _returnvalue_5 (.y (`self.InputAxes`))) (* (`KismetMathLibrary.Cross_VectorVector` _surfacenormal _returnvalue_5) (.x (`self.InputAxes`)))) 1.0))
  (set `self.StepOrigin` (`self.K2_GetActorLocation`))
  (set `self.SurfaceForward` _returnvalue_5)
  (set `self.StepCandidate` (+ (`self.StepOrigin`) (`self.StepDelta`)))
  (set `self.StepDelta` (* _returnvalue_6 (* (`self.SurfaceSpeed`) (`self.StepSeconds`))))
  (set `self.StepDirection` (`KismetMathLibrary.Normal` _returnvalue_6))
  (set `self.wallEdgeDetected` false)
  (`self.ProbeShadowSurface` (`self.StepOrigin`) (+ (`self.StepCandidate`) (* (`self.StepDirection`) (`self.SurfaceOffset`))))
  (if _probehit
    (`self.AcceptShadowContact`)
    (else
      (`self.ProbeShadowSurface` (+ (`self.StepCandidate`) _returnvalue) _returnvalue_3)
      (if _probehit
        (`self.AcceptShadowContact`)
        (else
          (`self.ProbeShadowSurface` _returnvalue_3 (- _returnvalue_4 (* (`self.StepDirection`) _probedepth)))
          (if _probehit
            (set `self.wallEdgeDetected` true)
            (`self.AcceptShadowContact`)
            (else
              (`self.ProbeShadowSurface` (+ (`self.StepOrigin`) _returnvalue) _returnvalue_4)
              (if _probehit
                (`self.AcceptShadowContact`)
                (else
                  (set `self.HasSurface` false)
                  (set `self.hasGround` false)
                  (set `self.isOnWall` false)
                  (set `self.wallDetected` false))))))))))

(fn `TickShadowSurface`
  (params (FrameSeconds :type "Float (double-precision)"))
  (bind _returnvalue (`KismetMathLibrary.FClamp` FrameSeconds 0.0 0.1))
  (bind _hassurface (`self.HasSurface`))
  (bind _surfacestepcount (`self.SurfaceStepCount`))
  (`|ExecutionSequence`
    (:`then_0`
      (if (not _hassurface)
        (`self.AcquireShadowSurface`)))
    (:`then_1`
      (if _hassurface
        (set `self.SurfaceStepCount` (`KismetMathLibrary.Clamp` (`KismetMathLibrary.FCeil` (`KismetMathLibrary.SafeDivide` (* _returnvalue (`self.SurfaceSpeed`)) (`KismetMathLibrary.FClamp` (`self.MaxSurfaceStep`) 1.0 40.0))) 1 64))
        (set `self.StepSeconds` (`KismetMathLibrary.SafeDivide` _returnvalue (`KismetMathLibrary.Conv_IntToDouble` _surfacestepcount)))
        (for _ (range _surfacestepcount)
          (`self.StepShadowSurface`))))))

(fn `UserConstructionScript`)